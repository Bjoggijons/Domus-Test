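; BP_Ai is an AI Blueprint that tracks player perception through state flags for seeing and searching.
; BeginPlay sets walk speed, caches the player and starts a looping timer for ChaseTick, which is not defined here.
; Perception updates set the flags per updated actor without checking whether sensing succeeded.
; On a player match, LastKnownPlayerLocation stores the AI's own location, not the player's.
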(event OnPerceptionUpdated(AIPerception)
  (params (UpdatedActors :type Array%20of%20Actor%20Object%20References))
  (for _array_element UpdatedActors
    (if (== _array_element (Variables|Default|GetPlayerRef))
      (Variables|Default|SetbCanSeePlayer true)
      (Variables|Default|SetbIsSearching false)
      (Variables|Default|SetLastKnownPlayerLocation (Transformation|GetActorLocation))
      (else
        (Variables|Default|SetbCanSeePlayer false)
        (Variables|Default|SetbIsSearching true)))))

(event EventBeginPlay
  (Variables|/Script/Engine.CharacterMovementComponent|SetMaxWalkSpeed (Variables|Character|GetCharacterMovement) (Variables|Default|GetSpeed))
  (Variables|Default|SetPlayerRef (Game|GetPlayerCharacter 0))
  (Utilities|Time|SetTimerbyFunctionName 0 "ChaseTick" 0.2 true))

(fn ConstructionScript)