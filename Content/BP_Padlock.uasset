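; BP_Padlock is a clickable combination padlock that opens a UI for entering a code.
; Clicking it creates WBP_PadlockUI, passes it a self reference, and switches to UI-only input with the cursor shown.
; UpdateCombination writes a digit into the current combination and compares the whole array to the correct one.
; A match only closes the widget and restores game input, with no further unlock action.
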(event OnClicked(combination_padlock)
  (params (TouchedComponent :type Primitive%20Component%20Object%20Reference) (ButtonPressed :type Key%20Structure :default "None"))
  (bind _returnvalue (Game|GetPlayerController 0))
  (bind _returnvalue_2 (UserInterface|CreateWidget "/Game/WBP_PadlockUI.WBP_PadlockUI_C" 0 0))
  (bind _output_get (Variables|Default|SetLockWidgetRef _returnvalue_2))
  (Variables|/Game/WBP_PadlockUI.WBP_PadlockUI_C|SetPadlockRef _output_get self)
  (UserInterface|Viewport|AddtoViewport _returnvalue_2 0)
  (Input|SetInputModeUIOnly _returnvalue _returnvalue_2 "DoNotLock" false)
  (Variables|/Script/Engine.PlayerController|SetbShowMouseCursor _returnvalue true))

(event Custom|UpdateCombination
  (params (NumberIndex :type Integer) (Value :type Integer))
  (Utilities|Array|SetArrayElem (Variables|Default|GetCurrentCombination) NumberIndex Value true)
  (CallFunction|CheckCombination))

(event Custom|CheckCombination
  (bind _returnvalue (Game|GetPlayerController 0))
  (for _index (range 0 2)
    (if (Utilities|Array|Identical (Variables|Default|GetCurrentCombination) (Variables|Default|GetCorrectCombination))
      _))
  (if (Utilities|Array|Identical (Variables|Default|GetCorrectCombination) (Variables|Default|GetCurrentCombination))
    (Widget|RemovefromParent (Variables|Default|GetLockWidgetRef))
    (Input|SetInputModeGameOnly _returnvalue false)
    (Variables|/Script/Engine.PlayerController|SetbShowMouseCursor _returnvalue false)))

(fn ConstructionScript)