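; BP_Book is a clickable bookshelf book that can act as the trigger for opening a hidden door.
; Interact_Book plays a timeline that slides the mesh from its starting relative location along the actor's forward vector by PullDistance.
; When the timeline finishes, a book flagged IsCorrectBook notifies BookshelfRef.
; Clicks call a separate Interact event, whose FlipFlop calls Interact again; nothing here calls Interact_Book.
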(event OnClicked(Book)
  (params (TouchedComponent :type Primitive%20Component%20Object%20Reference) (ButtonPressed :type Key%20Structure :default "None"))
  (CallFunction|Interact))

(event Custom|Interact_Book
  (bind _originallocation (Variables|Default|GetOriginalLocation))
  (bind _alpha (Timeline|Interact_Timeline Play)
    (:Update
      (Development|PrintString "Hello")
      (Transformation|SetRelativeLocation (Variables|Default|GetBook) (Math|Vector|Lerp(Vector) _originallocation (+ _originallocation (* (Transformation|GetActorForwardVector) (Variables|Default|GetPullDistance))) _alpha) false false))
    (:Finished
      (if (Variables|Default|GetIsCorrectBook)
        (Default|OnCorrectBookPulled (Variables|Default|GetBookshelfRef))
        (Development|PrintString "door opening")))))

(event EventInteract
  (Utilities|FlowControl|FlipFlop
    (:A
      (CallFunction|Interact)
      (Development|PrintString "right book"))))

(event EventBeginPlay
  (Variables|Default|SetOriginalLocation (Variables|/Script/Engine.SceneComponent|GetRelativeLocation (Variables|Default|GetBook))))

(fn ConstructionScript)