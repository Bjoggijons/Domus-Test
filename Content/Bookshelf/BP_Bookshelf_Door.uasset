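; Bookshelf door Blueprint that swings open when its OpenDoor event is called.
; BeginPlay caches the relative rotation, and OpenDoor plays a timeline whose alpha lerps from that rotation to the target.
; The target combines the cached rotation with a copy offset 90 degrees in yaw, so the original rotation counts twice and the swing is exactly 90 degrees only from a zero start.
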(event Custom|OpenDoor
  (bind _originalrotation (Variables|Default|GetOriginalRotation))
  (bind (_roll _pitch _yaw) (Math|Rotator|BreakRotator _originalrotation))
  (bind _alpha (Timeline|DoorOpenTimeline Play)
    (:Update
      (Transformation|SetRelativeRotation (Math|Rotator|Lerp(Rotator) _originalrotation (Math|Rotator|CombineRotators _originalrotation (Math|Rotator|MakeRotator _roll _pitch (+ _yaw 9e+01))) _alpha) false false))))

(event EventBeginPlay
  (Variables|Default|SetOriginalRotation (Variables|Default|GetRelativeRotation)))

(fn ConstructionScript)